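; Spawn volume actor that keeps spawning MyTarget_BP actors at random points inside its box.
; Tick feeds a one-second Delay, which ignores calls while pending, so it acts as a repeating timer of roughly one spawn per second.
; Each spawn location is a random offset within the Volume component's scaled extents added to the actor's location, ignoring the box's rotation.
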(event `self.ReceiveTick`
  (params (DeltaSeconds :type "Float (single-precision)"))
  (bind _x (.x (`BoxComponent.GetScaledBoxExtent` (`self.Volume`))))
  (bind _y (.y (`BoxComponent.GetScaledBoxExtent` (`self.Volume`))))
  (bind _z (.z (`BoxComponent.GetScaledBoxExtent` (`self.Volume`))))
  (`KismetSystemLibrary.Delay` 1.0)
  (`|SpawnActorFromClass` "/Game/Blueprints/Scene_Objects/MyTarget_BP.MyTarget_BP_C" (`KismetMathLibrary.Conv_VectorToTransform` (+ (`KismetMathLibrary.MakeVector` (`KismetMathLibrary.RandomFloatInRange` (* -1 _x) _x) (`KismetMathLibrary.RandomFloatInRange` (* -1 _y) _y) (`KismetMathLibrary.RandomFloatInRange` (* -1 _z) _z)) (`self.K2_GetActorLocation`))) "Undefined" "OverrideRootScale" null null))

(fn `UserConstructionScript`)